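; Base weapon Blueprint that sets up collision on its mesh and can create Chaos physics fields to break and push destructible objects.
; BeginPlay passes a valid WeaponMesh to InitializeCollisionForMesh.
; The CreateFields event hands a location to CreateFieldsSystem, which, if FieldSystem is valid, applies external cluster strain through a radial falloff, then linear force through a radial vector, both centred there.
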(event `self.ReceiveBeginPlay`
  (bind _weaponmesh (`self.WeaponMesh`)
    (:`then`
      (`self.InitializeCollisionForMesh` _weaponmesh))
    (:`else`)))

(event `self.CreateFields`
  (params (FieldLocation :type "Vector Structure (by ref)"))
  (`self.CreateFieldsSystem` FieldLocation))

(fn `CreateFieldsSystem`
  (params (`Field Location` :type "Vector Structure"))
  (locals (FieldLocation :type "Vector Structure"))
  (set `local.FieldLocation` `Field Location`)
  (bind _fieldsystem (`self.FieldSystem`)
    (:`then`
      (`FieldSystemComponent.ApplyPhysicsField` _fieldsystem true "Field_ExternalClusterStrain" null (`RadialFalloff.SetRadialFalloff` (`self.RadialFalloff`) 1000000.0 0.8 1.0 0.0 200.0 (`local.FieldLocation`) "Field_FallOff_None"))
      (`FieldSystemComponent.ApplyPhysicsField` _fieldsystem true "Field_LinearForce" (`self.FieldSystemMetaDataFilter`) (`RadialVector.SetRadialVector` (`self.RadialVector`) 15000.0 (`local.FieldLocation`))))
    (:`else`)))

(fn `UserConstructionScript`)